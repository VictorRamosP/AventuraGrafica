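; Player controller for a verb-based point-and-click adventure, moving the player character and running hotspot interactions.
; Left clicks path the character to a hotspot or ground point via AI MoveTo, storing the task so new clicks can cancel it.
; On arrival, the active verb calls its matching hotspot function.
; Task sequences (bark, face, wait) block hotspot hover changes, with face and wait advancing an index that re-triggers the interaction.
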(event `self.ReceiveBeginPlay`
  (`self.UpdateInteractionText`))

(event `Key|LeftMouseButton`
  (params (Key :type "Key Structure"))
  (:`Pressed`
    (`self.GetClick`
      (:`Hotspot`
        (`self.WalkToHotspot`
          (:`Out`
            (`self.Perform Interaction`))))
      (:`Nothing`
        (`self.ClearCurrentPath`)
        (`self.WalkToLocation`)))))

(event `Task Bark`
  (`/Game/Blueprints/BP_Player.PlayerBark` (`self.PlayerChar`) (`self.Bark Text`)))

(event `Task Face Direction`
  (`/Game/Blueprints/BP_Player.SetFacingDirection` (`self.PlayerChar`) (`self.Facing Direction`))
  (`KismetSystemLibrary.Delay` 0.2)
  (`self.IncrementTaskIndex`))

(event `Task Wait`
  (`KismetSystemLibrary.Delay` (`KismetMathLibrary.Conv_IntToDouble` (`self.WaitTime`)))
  (`self.IncrementTaskIndex`))

(fn `Assign Verb`
  (params (Verb :type "/Game/Blueprints/Enums/VerbUsed Enum" :default "NewEnumerator0"))
  (set `self.Active Verb` Verb)
  (`self.UpdateInteractionText`))

(fn `Begin Task Interaction`
  (set `self.Is Performing Task Interaction` true)
  (`self.IncrementTaskIndex`))

(fn `ClearCurrentPath`
  (bind _currentpath (`self.CurrentPath`))
  (`/Engine/EditorBlueprintResources/StandardMacros.IsValid` _currentpath
    (:`Is Valid`
      (`GameplayTask.EndTask` _currentpath))
    (:`Is Not Valid`
      _))
  (`self.InterruptAction`)
  (return))

(fn `End Task Interaction`
  (set `self.TaskIndex` 0)
  (set `self.Is Performing Task Interaction` false)
  (`self.InterruptAction`))

(fn `IncrementTaskIndex`
  (if (`self.Is Performing Task Interaction`)
    (`/Engine/EditorBlueprintResources/StandardMacros.IncrementInt` (`self.TaskIndex`)
      (:`  `
        (`self.Perform Interaction`)))))

(fn `InterruptAction`
  (`NavMovementInterface.StopActiveMovement` (`Character.CharacterMovement` (`self.PlayerChar`)))
  (set `self.Active Verb` "NewEnumerator0")
  (set `self.Target Hotspot` null)
  (set `self.Hotspot Interaction` false)
  (`self.Interrupting Action`))

(fn `Mouse Enter Hotspot`
  (params (Hotspot :type "/Game/Blueprints/Interactables/Base/BP_Hotspot Object Reference"))
  (if (not (or (`self.Is Performing Task Interaction`) (`self.Hotspot Interaction`)))
    (set `self.Target Hotspot` Hotspot)
    (`self.UpdateInteractionText`)))

(fn `Mouse Exit Hotspot`
  (if (not (or (`self.Is Performing Task Interaction`) (`self.Hotspot Interaction`)))
    (set `self.Target Hotspot` null)
    (`self.UpdateInteractionText`)))

(fn `UserConstructionScript`)