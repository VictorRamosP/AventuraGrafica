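; Blueprint function library of global shortcuts for the game's HUD, game instance, player controller, player character and room transitions.
; Getters cast to the project classes or find the top-level HUD widget, and most other functions build on them.
; Room loading is delegated to game instance events, with the used door stored first.
; Other helpers toggle the player input lock and black screen, and have the player assign the room camera.
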(fn `Activate Current Camera`
  (`/Game/Blueprints/BP_Player.Assing Room Camera` (`self.GetPlayer` null)))

(fn `GetGameInstance`
  (returns (GameInstance :type "/Game/Blueprints/BP_GameInstance Object Reference"))
  (bind _asbp_game_instance (cast `/Game/Blueprints/BP_GameInstance` (`GameplayStatics.GetGameInstance` null)))
  (return _asbp_game_instance))

(fn `GetHUD`
  (returns (HUD :type "/Game/Blueprints/Widgets/WBP_HUD Object Reference"))
  (bind _foundwidgets (`WidgetBlueprintLibrary.GetAllWidgetsOfClass` null "/Game/Blueprints/Widgets/WBP_HUD.WBP_HUD_C"))
  (return (`|GetArrayItem` _foundwidgets)))

(fn `GetPlayer`
  (returns (Player :type "/Game/Blueprints/BP_Player Object Reference"))
  (bind _asbp_player_controller (cast `/Game/Blueprints/BP_PlayerController` (`GameplayStatics.GetPlayerController` null)))
  (return (`/Game/Blueprints/BP_PlayerController.PlayerChar` _asbp_player_controller)))

(fn `GetPlayerController`
  (returns (`Player Controller` :type "/Game/Blueprints/BP_PlayerController Object Reference"))
  (bind _asbp_player_controller (cast `/Game/Blueprints/BP_PlayerController` (`GameplayStatics.GetPlayerController` null)))
  (return _asbp_player_controller))

(fn `Hide Black Screen`
  (`Widget.SetVisibility` (`/Game/Blueprints/Widgets/WBP_HUD.BlackScreen` (`self.GetHUD` null)) "Hidden"))

(fn `LoadRoom`
  (params (DoorUsed :type "/Game/Blueprints/Interactables/BP_Hotspot_Door Object Reference"))
  (bind _gameinstance (`self.GetGameInstance` null))
  (set `/Game/Blueprints/BP_GameInstance.CurrentDoor` DoorUsed _gameinstance)
  (`/Game/Blueprints/BP_GameInstance.Event Load Room` _gameinstance))

(fn `LoadStartingRoom`
  (`/Game/Blueprints/BP_GameInstance.Event Load Starting Room` (`self.GetGameInstance` null)))

(fn `Lock Player Input`
  (set `/Game/Blueprints/BP_PlayerController.LockInput` true (`self.GetPlayerController` null)))

(fn `Show Black Screen`
  (`Widget.SetVisibility` (`/Game/Blueprints/Widgets/WBP_HUD.BlackScreen` (`self.GetHUD` null)) "Visible"))

(fn `UnlockPlayerInput`
  (set `/Game/Blueprints/BP_PlayerController.LockInput` false (`self.GetPlayerController` null)))