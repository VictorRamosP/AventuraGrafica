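; BP_Npc is an interactable NPC that shows one line of dialogue per interaction.
; Each Interact event increments IndexDialogue and, while it is at most the dialogue array's length, writes that entry to a Wb_Dialogue widget's text.
; The widget is created for player 0 and added to the viewport when no valid one exists, then reused; this graph never removes it or resets the index.
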(event `/Game/Blueprints/Dialogue/BP_Interface.Interact`
  (`/Engine/EditorBlueprintResources/StandardMacros.IncrementInt` (`self.IndexDialogue`)
    (:`  `
      (if (<= (`self.IndexDialogue`) (`KismetArrayLibrary.Array_Length` (`self.Diaolgue`)))
        (`self.Ui`
          (:`then`
            _)
          (:`else`
            (bind _returnvalue (`|CreateWidget` "/Game/Blueprints/Dialogue/Wb_Dialogue.Wb_Dialogue_C" (`GameplayStatics.GetPlayerController` 0)))
            (bind _output_get (set `self.Ui` _returnvalue))
            (`UserWidget.AddToViewport` _output_get 0)))
        (`TextBlock.SetText` (`/Game/Blueprints/Dialogue/Wb_Dialogue.DialogueText` (`self.Ui`)) (`KismetTextLibrary.Conv_StringToText` (`|GetArrayItem` (`self.Diaolgue`) (`self.IndexDialogue`))))))))

(fn `UserConstructionScript`)