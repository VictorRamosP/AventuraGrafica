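; Camera actor that smoothly follows the Player on X and Y inside a box of confines, keeping its own Z.
; Construction sizes the box; BeginPlay derives clamp limits from its bounds, inset by half OrthoWidth on X but only the AspectRatio value on Y.
; Each Tick interpolates toward the player's capsule, clamps to those limits and moves the camera, or prints a warning if Player is invalid.
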(event `self.ReceiveBeginPlay`
  ;[0 0 0 0.5] Set Camera as main
  (`self.GetCameraConfines`))

(event `self.ReceiveTick`
  (params (DeltaSeconds :type "Float (single-precision)"))
  (set `self.DeltaSeconds` DeltaSeconds)
  (`/Engine/EditorBlueprintResources/StandardMacros.IsValid` (`self.Player`)
    (:`Is Valid`
      ;[0 0 0 0.5] Follow Player
      (`self.CamFollowPlayerX`
        (:`Out`
          (`self.CamFollowPlayerY`
            (:`Out`
              (`self.LerpWithinConfines`
                (:`Out`
                  (`self.SetCameraLocation`))))))))
    (:`Is Not Valid`
      (`KismetSystemLibrary.PrintString` "PlayerNotValid"))))

(fn `UserConstructionScript`
  ;[0 0 0 0.5] Setea el tamanyo de la cámara
  (`BoxComponent.SetBoxExtent` (`self.CameraConfines`) (`self.ConfinesExtent`) true))