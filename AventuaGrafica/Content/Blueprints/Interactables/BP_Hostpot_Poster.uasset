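; Poster hotspot interactable that plays a short scripted look-at interaction.
; OnLookat switches on the PlayerController's TaskIndex to run one step: begin the task, face the hotspot, bark a remark, face a set direction, then bark again.
; Any other index ends the task interaction.
; The construction script only calls its parent.
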(event `/Game/Blueprints/Interactables/Base/BPI_VerbInteraction.OnLookAt`
  (switch `int` (`/Game/Blueprints/BP_PlayerController.TaskIndex` (`self.PlayerController`))
    (:`Default`
      (`self.EndTaskInteraction`))
    (:`0`
      (`self.Begin Task Interaction`))
    (:`1`
      (`self.FaceHotspot`))
    (:`2`
      (`self.Bark` "Looks like a poster to me."))
    (:`3`
      (`self.Face Direction` "NewEnumerator3"))
    (:`4`
      (`self.Bark` "Wow, what a nice poster."))))

(fn `UserConstructionScript`
  (`parent.UserConstructionScript`))