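; NPC hotspot for a dialogue interaction, playing a short scripted comedic greeting when talked to.
; OnTalkto shows the HUD dialog and switches on the player controller's task index to begin the interaction, turn, show lines, bark or end.
; Spoken text steps share a three-second delay before incrementing the task index, while the bark and end steps hide the dialog.
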(event `/Game/Blueprints/Interactables/Base/BPI_VerbInteraction.OnTalkTo`
  (bind _hud (`/Game/Blueprints/BFL_GameLibrary.GetHUD`))
  (`/Game/Blueprints/Widgets/WBP_HUD.ShowDialog` _hud)
  (switch `int` (`/Game/Blueprints/BP_PlayerController.TaskIndex` (`self.PlayerController`))
    (:`0`
      (`self.Begin Task Interaction`))
    (:`1`
      (`self.FaceHotspot`))
    (:`2`
      (`/Game/Blueprints/Widgets/WBP_HUD.ShowText` _hud "Welcome to my nudist island!")
      (`KismetSystemLibrary.Delay` 3.0 :!label _label)
      (`/Game/Blueprints/BP_PlayerController.IncrementTaskIndex` (`/Game/Blueprints/BFL_GameLibrary.GetPlayerController`)))
    (:`3`
      (`/Game/Blueprints/Widgets/WBP_HUD.ShowText` _hud "Be careful with your rear")
      (goto _label))
    (:`4`
      (`/Game/Blueprints/Widgets/WBP_HUD.ShowText` _hud "Enjoy! *wink*")
      (goto _label))
    (:`5`
      (`self.Face Direction` "NewEnumerator3"))
    (:`6`
      (`self.Bark` "I should have brought vaseline")
      (`/Game/Blueprints/Widgets/WBP_HUD.OcultDialog` _hud :!label _label_2))
    (:`7`
      (`self.EndTaskInteraction`)
      (goto _label_2))))

(fn `UserConstructionScript`
  (`parent.UserConstructionScript`))