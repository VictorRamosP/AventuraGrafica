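; BP_Hotspot is the base interactable for point-and-click adventure verbs.
; Its static mesh's cursor-over events notify BP_PlayerController when the mouse enters or exits the hotspot.
; Overridable interface events for the nine verbs, such as Look at, Use and Pick up, print default refusal lines.
; The construction script places the WalkToPoint component at the WalkToPosition world location.
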(event `self.StaticMeshComponent.OnBeginCursorOver`
  (params (TouchedComponent :type "PrimitiveComponent Object Reference"))
  ;[0 0 0 0.5] Cuando el Hotspot detecta que le pasan el mouse por encima llama a la funcion en el PlayerController
  (bind _asbp_player_controller (cast `/Game/Blueprints/BP_PlayerController` (`GameplayStatics.GetPlayerController` 0)))
  (`/Game/Blueprints/BP_PlayerController.Mouse Enter Hotspot` _asbp_player_controller self))

(event `self.StaticMeshComponent.OnEndCursorOver`
  (params (TouchedComponent :type "PrimitiveComponent Object Reference"))
  ;[0 0 0 0.5] Cuando el Hotspot detecta que le pasan el mouse por encima llama a la funcion en el PlayerController
  (bind _asbp_player_controller (cast `/Game/Blueprints/BP_PlayerController` (`GameplayStatics.GetPlayerController` 0)))
  (`/Game/Blueprints/BP_PlayerController.Mouse Exit Hotspot` _asbp_player_controller))

(event `/Game/Blueprints/Interactables/Base/BPI_VerbInteraction.OnPull`
  ;[0 0 0 0.5] Implementa una interface para poder sobreescribir las funciones
  ;;[0 0 0 0.5] Interacciones default para los objetos
  (`KismetSystemLibrary.PrintString` "It won't move."))

(event `/Game/Blueprints/Interactables/Base/BPI_VerbInteraction.OnPush`
  ;[0 0 0 0.5] Implementa una interface para poder sobreescribir las funciones
  ;;[0 0 0 0.5] Interacciones default para los objetos
  (`KismetSystemLibrary.PrintString` "I can't push that."))

(event `/Game/Blueprints/Interactables/Base/BPI_VerbInteraction.OnUse`
  ;[0 0 0 0.5] Implementa una interface para poder sobreescribir las funciones
  ;;[0 0 0 0.5] Interacciones default para los objetos
  (`KismetSystemLibrary.PrintString` "I can't use that."))

(event `/Game/Blueprints/Interactables/Base/BPI_VerbInteraction.OnTalkTo`
  ;[0 0 0 0.5] Implementa una interface para poder sobreescribir las funciones
  ;;[0 0 0 0.5] Interacciones default para los objetos
  (`KismetSystemLibrary.PrintString` "It doesn't want to listen."))

(event `/Game/Blueprints/Interactables/Base/BPI_VerbInteraction.OnLookAt`
  ;[0 0 0 0.5] Implementa una interface para poder sobreescribir las funciones
  ;;[0 0 0 0.5] Interacciones default para los objetos
  (`KismetSystemLibrary.PrintString` "I see nothing interesting there."))

(event `/Game/Blueprints/Interactables/Base/BPI_VerbInteraction.OnClose`
  ;[0 0 0 0.5] Implementa una interface para poder sobreescribir las funciones
  ;;[0 0 0 0.5] Interacciones default para los objetos
  (`KismetSystemLibrary.PrintString` "Can't close that."))

(event `/Game/Blueprints/Interactables/Base/BPI_VerbInteraction.OnOpen`
  ;[0 0 0 0.5] Implementa una interface para poder sobreescribir las funciones
  ;;[0 0 0 0.5] Interacciones default para los objetos
  (`KismetSystemLibrary.PrintString` "Won't open."))

(event `/Game/Blueprints/Interactables/Base/BPI_VerbInteraction.OnGive`
  ;[0 0 0 0.5] Implementa una interface para poder sobreescribir las funciones
  ;;[0 0 0 0.5] Interacciones default para los objetos
  (`KismetSystemLibrary.PrintString` "I can't give that."))

(event `/Game/Blueprints/Interactables/Base/BPI_VerbInteraction.OnPickup`
  ;[0 0 0 0.5] Implementa una interface para poder sobreescribir las funciones
  ;;[0 0 0 0.5] Interacciones default para los objetos
  (`KismetSystemLibrary.PrintString` "I can't pick that up."))

(fn `UserConstructionScript`
  (`SceneComponent.K2_SetWorldLocation` (`self.WalkToPoint`) (`self.WalkToPosition`) false false))